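; MeleeHit is an animation notify state that opens a melee hit window during an attack animation.
; On begin, it casts the mesh owner to ThirdPersonCharacter and sets its MeleeAttackHit component to query-only collision.
; On end, it turns that collision off, so hits can register only during the notify's span.
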(fn `Received_NotifyBegin`
  (params (MeshComp :type "SkeletalMeshComponent Object Reference") (Animation :type "AnimSequenceBase Object Reference") (TotalDuration :type "Float (double-precision)"))
  (returns (ReturnValue :type Boolean))
  ;[1 1 1] At this point in the animation, the attack collision is enabled.
  (`PrimitiveComponent.SetCollisionEnabled` (`/Game/StarterContent/ThirdPersonBP/Blueprints/ThirdPersonCharacter.MeleeAttackHit` (cast `/Game/StarterContent/ThirdPersonBP/Blueprints/ThirdPersonCharacter` (`ActorComponent.GetOwner` MeshComp) :!pure true)) "QueryOnly")
  (return false))

(fn `Received_NotifyEnd`
  (params (MeshComp :type "SkeletalMeshComponent Object Reference") (Animation :type "AnimSequenceBase Object Reference"))
  (returns (ReturnValue :type Boolean))
  ;[1 1 1] At this point in the animation, the attack collision is disabled
  (`PrimitiveComponent.SetCollisionEnabled` (`/Game/StarterContent/ThirdPersonBP/Blueprints/ThirdPersonCharacter.MeleeAttackHit` (cast `/Game/StarterContent/ThirdPersonBP/Blueprints/ThirdPersonCharacter` (`ActorComponent.GetOwner` MeshComp) :!pure true)) "NoCollision")
  (return false))
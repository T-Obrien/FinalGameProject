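; Anim notify state that stops a FollowerCharacter from walking for the span of the notify in an animation.
; On begin it casts the mesh owner to FollowerCharacter and zeroes the movement component's MaxWalkSpeed.
; On end it sets a hard-coded walk speed rather than restoring the previous value.
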(fn `Received_NotifyBegin`
  (params (MeshComp :type "SkeletalMeshComponent Object Reference") (Animation :type "AnimSequenceBase Object Reference") (TotalDuration :type "Float (double-precision)"))
  (returns (ReturnValue :type Boolean))
  (set `CharacterMovementComponent.MaxWalkSpeed` 0.0 (`Character.CharacterMovement` (cast `/Game/Blueprints/AI/FollowerCharacter` (`ActorComponent.GetOwner` MeshComp) :!pure true)))
  (return false))

(fn `Received_NotifyEnd`
  (params (MeshComp :type "SkeletalMeshComponent Object Reference") (Animation :type "AnimSequenceBase Object Reference"))
  (returns (ReturnValue :type Boolean))
  (set `CharacterMovementComponent.MaxWalkSpeed` 250.0 (`Character.CharacterMovement` (cast `/Game/Blueprints/AI/FollowerCharacter` (`ActorComponent.GetOwner` MeshComp) :!pure true)))
  (return false))
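; Ranger enemy that alternates between moving to random nearby navigable points and firing frostbolts, looping until death.
; Each attack snaps yaw toward the player once, then times the projectile spawn and return to movement with delays matched to the cast animation.
; Damage updates a widget health bar, shown only while the player overlaps its display zone.
; At zero health it plays a death animation, disables capsule collision and destroys itself after a delay.
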(event `self.ReceiveBeginPlay`
  (bind _asranger_enemy_health (cast `/Game/UI/RangerEnemyHealth` (`WidgetComponent.GetUserWidgetObject` (`self.RangerHealthBar`))))
  (set `self.UI_HealthBar` _asranger_enemy_health)
  (`self.MoveRandomLocation`))

(event `MoveRandomLocation`
  ;[1 1 1] The enemy picks a spot in range, and travels towards it
  (if (not (`self.IsDead`))
    (`|AIMoveTo` self (`NavigationSystemV1.K2_GetRandomLocationInNavigableRadius` (`self.K2_GetActorLocation`) (`KismetMathLibrary.RandomFloatInRange` 400.0 900.0) null null) null
      (:`OnSuccess`
        (`KismetSystemLibrary.Delay` 0.1)
        (`self.FireProjectile`)))))

(event `self.UI_DisplayZone.OnComponentBeginOverlap`
  (params (OverlappedComponent :type "PrimitiveComponent Object Reference") (OtherActor :type "Actor Object Reference") (OtherComp :type "PrimitiveComponent Object Reference") (OtherBodyIndex :type Integer) (bFromSweep :type Boolean) (SweepResult :type "HitResult Structure (by ref)"))
  (cast `/Game/StarterContent/ThirdPersonBP/Blueprints/ThirdPersonCharacter` OtherActor)
  (`SceneComponent.SetVisibility` (`self.RangerHealthBar`) true false))

(event `self.UI_DisplayZone.OnComponentEndOverlap`
  (params (OverlappedComponent :type "PrimitiveComponent Object Reference") (OtherActor :type "Actor Object Reference") (OtherComp :type "PrimitiveComponent Object Reference") (OtherBodyIndex :type Integer))
  (cast `/Game/StarterContent/ThirdPersonBP/Blueprints/ThirdPersonCharacter` OtherActor)
  (`SceneComponent.SetVisibility` (`self.RangerHealthBar`) false false))

(event `FireProjectile`
  ;[1 1 1] At the start of the attack, the enemy faces towards the player and begins the animation. Part-way through the animation, the projectile is fired. Then the animation finishes and the enemy can move again
  (if (not (`self.IsDead`))
    (set `self.ShouldFacePlayer` true)
    (bind _asthird_person_character (cast `/Game/StarterContent/ThirdPersonBP/Blueprints/ThirdPersonCharacter` (`GameplayStatics.GetPlayerCharacter` 0)))
    (set `self.Char Ref` _asthird_person_character)
    (`self.FaceTowardsPlayer`)
    (if (not (`self.IsDead`))
      (set `self.ShouldFacePlayer` false)
      (`SkeletalMeshComponent.PlayAnimation` (`self.Mesh`) "/Game/Animation/RangerEnemy/Standing_2H_Magic_Attack_02.Standing_2H_Magic_Attack_02" false)
      (`KismetSystemLibrary.Delay` 1.48952)
      (if (not (`self.IsDead`))
        (`|SpawnActorFromClass` "/Game/Blueprints/AI/RangerFrostbolt.RangerFrostbolt_C" (`KismetMathLibrary.MakeTransform` (`SceneComponent.K2_GetComponentLocation` (`self.FrostboltSpawnPoint`)) (`self.K2_GetActorRotation`)) "Undefined" "OverrideRootScale" null null)
        (`KismetSystemLibrary.Delay` 1.377147)
        (if (not (`self.IsDead`))
          (`SkeletalMeshComponent.SetAnimationMode` (`self.Mesh`) "AnimationBlueprint")
          (`self.MoveRandomLocation`))))))

(event `FaceTowardsPlayer`
  (bind (_returnvalue_roll _returnvalue_pitch _returnvalue_yaw) (`KismetMathLibrary.BreakRotator` (`KismetMathLibrary.RInterpTo` (`self.K2_GetActorRotation`) (`KismetMathLibrary.FindLookAtRotation` (`self.K2_GetActorLocation`) (`self.K2_GetActorLocation` (`self.Char Ref`))) (`GameplayStatics.GetWorldDeltaSeconds`) 9000.0)))
  ;[1 1 1] When aiming their attack, the enemy looks towards the player's location
  (if (`self.IsDead`)
    _
    (elif (`self.ShouldFacePlayer`)
      (`self.K2_SetActorRotation` (`KismetMathLibrary.MakeRotator` 0.0 0.0 _returnvalue_yaw)))))

(event `self.ReceiveAnyDamage`
  (params (Damage :type "Float (single-precision)") (DamageType :type "DamageType Object Reference") (InstigatedBy :type "Controller Object Reference") (DamageCauser :type "Actor Object Reference"))
  (`KismetSystemLibrary.PrintString` (`KismetStringLibrary.Conv_DoubleToString` Damage))
  (bind _output_get (set `self.Health` (- (`self.Health`) Damage)))
  (set `/Game/UI/RangerEnemyHealth.DisplayedHealth` _output_get (`self.UI_HealthBar`))
  (if (<= (`self.Health`) 0.0)
    (set `self.IsDead` true)
    (`SkeletalMeshComponent.SetAnimationMode` (`self.Mesh`) "AnimationSingleNode")
    (`SkeletalMeshComponent.PlayAnimation` (`self.Mesh`) "/Game/Animation/RangerEnemy/Death_Crouching_Headshot_Front.Death_Crouching_Headshot_Front" false)
    (`PrimitiveComponent.SetCollisionEnabled` (`self.CapsuleComponent`) "NoCollision")
    (`KismetSystemLibrary.Delay` 5.5)
    (`self.K2_DestroyActor`)))

(fn `UserConstructionScript`)
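; Zombie enemy character that chases player 0, deals damage on contact and dies when its health drops below zero.
; A self-calling chase event reissues AI MoveTo and refreshes player distance, which Tick checks to toggle a timed IsAttacking flag.
; Damage comes from DamageBox overlaps with Player-tagged actors, independent of that flag.
; Death plays an animation, disables capsule collision and destroys the actor after a delay.
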(event `self.ReceiveAnyDamage`
  (params (Damage :type "Float (single-precision)") (DamageType :type "DamageType Object Reference") (InstigatedBy :type "Controller Object Reference") (DamageCauser :type "Actor Object Reference"))
  ;[1 1 1] When it takes damage, the enemy's health changes. If it is below zero, the enemy dies.
  (`KismetSystemLibrary.PrintString` (`KismetStringLibrary.Conv_DoubleToString` Damage))
  (set `self.Health` (- (`self.Health`) Damage))
  (if (< (`self.Health`) 0.0)
    (`SkeletalMeshComponent.SetAnimationMode` (`self.Mesh`) "AnimationSingleNode")
    (`SkeletalMeshComponent.PlayAnimation` (`self.Mesh`) "/Game/Animation/FollowerEnemy/Zombie_Dying.Zombie_Dying" false)
    (set `self.IsDead` true)
    (`PrimitiveComponent.SetCollisionEnabled` (`self.CapsuleComponent`) "NoCollision")
    (`KismetSystemLibrary.Delay` 5.5)
    (`self.K2_DestroyActor`)))

(event `self.ReceiveBeginPlay`
  ;[1 1 1] Comment
  (`self.ChasePlayer`))

(event `ChasePlayer`
  (bind _returnvalue (`GameplayStatics.GetPlayerCharacter` 0))
  ;[1 1 1] Comment
  (if (not (`self.IsDead`))
    (`|AIMoveTo` self (0.0 0.0 0.0) _returnvalue
      (:`then`
        (`KismetSystemLibrary.Delay` 0.2)
        (set `self.AttackDistance` (`self.GetDistanceTo` _returnvalue))
        (`self.ChasePlayer`)))))

(event `self.ReceiveTick`
  (params (DeltaSeconds :type "Float (single-precision)"))
  (if (`self.IsAttacking`)
    _
    (elif (<= (`self.AttackDistance`) 130.0)
      (`self.AttackPlayer`))))

(event `AttackPlayer`
  (set `self.IsAttacking` true)
  (`KismetSystemLibrary.Delay` 3.2)
  (set `self.IsAttacking` false))

(event `self.DamageBox.OnComponentBeginOverlap`
  (params (OverlappedComponent :type "PrimitiveComponent Object Reference") (OtherActor :type "Actor Object Reference") (OtherComp :type "PrimitiveComponent Object Reference") (OtherBodyIndex :type Integer) (bFromSweep :type Boolean) (SweepResult :type "HitResult Structure (by ref)"))
  (if (`self.ActorHasTag` OtherActor "Player")
    (`GameplayStatics.ApplyDamage` OtherActor 15.0 null self)))

(fn `UserConstructionScript`)
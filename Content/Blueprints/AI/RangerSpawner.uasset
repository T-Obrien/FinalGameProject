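; Ranger spawner actor that keeps RangerCharacter enemies spawning at random points inside its box, scaled to the current round.
; Each tick it reads RoundNumber from the RoundCount actor and sets the enemy cap, cooldown and double-spawn flag for rounds two through five.
; While the live ranger count is below the cap, it waits out the cooldown, then spawns one, or two once double spawn is enabled.
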(event `self.ReceiveTick`
  (params (DeltaSeconds :type "Float (single-precision)"))
  (bind _box (`self.Box`))
  (bind _box_2 (`self.Box`))
  (`self.Check Round Number`)
  (bind _outactors (`GameplayStatics.GetAllActorsOfClass` "/Game/Blueprints/AI/RangerCharacter.RangerCharacter_C"))
  (if (< (`KismetArrayLibrary.Array_Length` _outactors) (`self.MaxEnemies`))
    (`KismetSystemLibrary.Delay` (`self.SpawnCooldown`))
    (`AIBlueprintHelperLibrary.SpawnAIFromClass` "/Game/Blueprints/AI/RangerCharacter.RangerCharacter_C" null (`KismetMathLibrary.RandomPointInBoundingBox` (`SceneComponent.K2_GetComponentLocation` _box_2) (`BoxComponent.GetScaledBoxExtent` _box_2)) (struct) false null)
    (if (`self.CanDoubleSpawn`)
      (`AIBlueprintHelperLibrary.SpawnAIFromClass` "/Game/Blueprints/AI/RangerCharacter.RangerCharacter_C" null (`KismetMathLibrary.RandomPointInBoundingBox` (`SceneComponent.K2_GetComponentLocation` _box) (`BoxComponent.GetScaledBoxExtent` _box)) (struct) false null))))

(event `Check Round Number`
  (bind _outactors (`GameplayStatics.GetAllActorsOfClass` "/Game/Blueprints/AI/RoundCount.RoundCount_C"))
  (bind _asround_count (cast `/Game/Blueprints/AI/RoundCount` (`|GetArrayItem` _outactors)))
  (bind _round_number (`/Game/Blueprints/AI/RoundCount.Round Number` _asround_count))
  (if (== _round_number 1)
    _
    (elif (== _round_number 2)
      (set `self.MaxEnemies` 3)
      (set `self.SpawnCooldown` 7.0)
      (elif (== _round_number 3)
        (set `self.MaxEnemies` 5)
        (set `self.SpawnCooldown` 6.0)
        (elif (== _round_number 4)
          (set `self.MaxEnemies` 6)
          (set `self.SpawnCooldown` 4.5)
          (elif (== _round_number 5)
            (set `self.MaxEnemies` 8)
            (set `self.SpawnCooldown` 5.5)
            (set `self.CanDoubleSpawn` true)))))))

(fn `UserConstructionScript`)
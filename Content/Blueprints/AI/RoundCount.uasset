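; RoundCount is an AI Blueprint that derives the current round number from the enemy kill count.
; Each Tick, nested branches compare EnemyKillCount against fixed, rising thresholds and set RoundNumber to a value from one to five.
; The round is recomputed every frame by polling, and the construction script is empty.
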(event `self.ReceiveTick`
  (params (DeltaSeconds :type "Float (single-precision)"))
  (if (>= (`self.EnemyKillCount`) 4)
    (if (>= (`self.EnemyKillCount`) 9)
      (if (>= (`self.EnemyKillCount`) 14)
        (if (>= (`self.EnemyKillCount`) 20)
          (set `self.Round Number` 5)
          (else
            (set `self.Round Number` 4)))
        (else
          (set `self.Round Number` 3)))
      (else
        (set `self.Round Number` 2)))
    (else
      (set `self.Round Number` 1))))

(fn `UserConstructionScript`)
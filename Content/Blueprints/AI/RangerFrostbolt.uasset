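; RangerFrostbolt is a projectile actor that flies straight along its forward vector and explodes on impact.
; A looping timer started on BeginPlay moves it a fixed step at roughly 60 Hz, without sweeping.
; Its Sphere overlap reacts to actors tagged Player or DestroyProj, applying damage to either, spawning a RangerFrostboltExplosion at its transform and destroying itself.
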(event `self.ReceiveBeginPlay`
  (`KismetSystemLibrary.K2_SetTimer` null "MoveForward" 0.016667 true))

(event `MoveForward`
  (`self.K2_SetActorLocation` (+ (`self.K2_GetActorLocation`) (* (`self.GetActorForwardVector`) 7.5))))

(event `self.Sphere.OnComponentBeginOverlap`
  (params (OverlappedComponent :type "PrimitiveComponent Object Reference") (OtherActor :type "Actor Object Reference") (OtherComp :type "PrimitiveComponent Object Reference") (OtherBodyIndex :type Integer) (bFromSweep :type Boolean) (SweepResult :type "HitResult Structure (by ref)"))
  (if (`self.ActorHasTag` OtherActor "Player")
    (`GameplayStatics.ApplyDamage` OtherActor 25.0 null self :!label _label)
    (`|SpawnActorFromClass` "/Game/Blueprints/AI/RangerFrostboltExplosion.RangerFrostboltExplosion_C" (`self.GetTransform`) "Undefined" "OverrideRootScale" null null)
    (`self.K2_DestroyActor`)
    (elif (`self.ActorHasTag` OtherActor "DestroyProj")
      (goto _label))))

(fn `UserConstructionScript`)
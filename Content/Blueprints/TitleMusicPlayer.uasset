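; Actor that plays the title screen music and stops it when the player character signals it.
; On BeginPlay it finds the ThirdPersonCharacter, caches it, and spawns TitleScreenMusicV1 as a 2D sound.
; Every Tick it polls the character's StopMusic flag; once set, it deactivates the audio component and destroys itself.
; An unconnected StopPlaying branch remains unused.
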(event `self.ReceiveBeginPlay`
  (bind _returnvalue (`GameplayStatics.GetActorOfClass` "/Game/StarterContent/ThirdPersonBP/Blueprints/ThirdPersonCharacter.ThirdPersonCharacter_C"))
  (set `self.Char Ref` _returnvalue)
  (bind _returnvalue_2 (`GameplayStatics.SpawnSound2D` "/Game/Sound/TitleScreenMusicV1.TitleScreenMusicV1" 1.0 1.0 0.0 null)))

(event `self.ReceiveTick`
  (params (DeltaSeconds :type "Float (single-precision)"))
  (if (`/Game/StarterContent/ThirdPersonBP/Blueprints/ThirdPersonCharacter.StopMusic` (`self.Char Ref`))
    (`ActorComponent.SetActive` (stale `self.ReceiveBeginPlay` _returnvalue_2) false false)
    (`self.K2_DestroyActor`)))

(fn `UserConstructionScript`)
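; BP_SpectatorSitting1 is a seated crowd spectator that celebrates when a RoundCount actor flags it.
; Tick polls that actor's ShouldCelebrate, swaps the static mesh to a celebrating pose, then restores a sitting mesh after a delay and clears the flag.
; Cheer cycles through three timed variants, setting the delay length and using CanCheer to block re-triggering while one runs.
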(event `Cheer`
  (bind _cheercount (`self.CheerCount`))
  (if (== (`self.CanCheer`) true)
    (if (== _cheercount 1)
      (set `self.CanCheer` false)
      (bind _output_get (set `self.CheerDelay` 4.133333))
      (`KismetSystemLibrary.Delay` _output_get)
      (set `self.CheerCount` 2)
      (set `self.CanCheer` true)
      (elif (== _cheercount 2)
        (set `self.CanCheer` false)
        (bind _output_get_2 (set `self.CheerDelay` 7.0))
        (`KismetSystemLibrary.Delay` _output_get_2)
        (set `self.CheerCount` 3)
        (set `self.CanCheer` true)
        (else
          (set `self.CanCheer` false)
          (bind _output_get_3 (set `self.CheerDelay` 6.7))
          (`KismetSystemLibrary.Delay` _output_get_3)
          (set `self.CheerCount` 1)
          (set `self.CanCheer` true))))))

(event `self.ReceiveTick`
  (params (DeltaSeconds :type "Float (single-precision)"))
  (bind _returnvalue (`GameplayStatics.GetActorOfClass` "/Game/Blueprints/AI/RoundCount.RoundCount_C"))
  (if (`/Game/Blueprints/AI/RoundCount.ShouldCelebrate` _returnvalue)
    (`StaticMeshComponent.SetStaticMesh` (`self.Spectator`) "/Game/Models/Environment/SittingCelebratorV1.SittingCelebratorV1")
    (`self.Cheer`)
    (`KismetSystemLibrary.Delay` (`self.CheerDelay`))
    (`StaticMeshComponent.SetStaticMesh` (`self.Spectator`) "/Game/Models/Environment/SittingSpectatorV2.SittingSpectatorV2")
    (bind _returnvalue_2 (`GameplayStatics.GetActorOfClass` "/Game/Blueprints/AI/RoundCount.RoundCount_C"))
    (set `/Game/Blueprints/AI/RoundCount.ShouldCelebrate` false _returnvalue_2)))

(fn `UserConstructionScript`)
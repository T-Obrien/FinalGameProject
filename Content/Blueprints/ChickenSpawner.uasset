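; Spawner actor that places a HealthChicken at a random point inside its Box component's bounds.
; Tick calls SpawnChicken while CanSpawn is true, which clears the flag and spawns the chicken after a 30-second delay.
; Nothing in this Blueprint sets CanSpawn back to true, so any further spawn depends on the flag being set elsewhere.
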(event `SpawnChicken`
  (bind _box (`self.Box`))
  (set `self.CanSpawn` false)
  (`KismetSystemLibrary.Delay` 30.0)
  (`|SpawnActorFromClass` "/Game/Blueprints/HealthChicken.HealthChicken_C" (`KismetMathLibrary.MakeTransform` (`KismetMathLibrary.RandomPointInBoundingBox` (`SceneComponent.K2_GetComponentLocation` _box) (`BoxComponent.GetScaledBoxExtent` _box))) "Undefined" "OverrideRootScale" null null))

(event `self.ReceiveTick`
  (params (DeltaSeconds :type "Float (single-precision)"))
  (if (`self.CanSpawn`)
    (`self.SpawnChicken`)))

(fn `UserConstructionScript`)
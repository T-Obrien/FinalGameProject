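; Spear pickup that shows an equip prompt when the third-person character comes close.
; Entering the UI_DisplayZone overlap volume sets the character's NearSpear flag and reveals PickupUI, unless WeaponMode indicates a spear is already held.
; Leaving the zone clears the flag and hides the prompt.
; The Blueprint only signals proximity and contains no equip logic.
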(event `self.UI_DisplayZone.OnComponentBeginOverlap`
  (params (OverlappedComponent :type "PrimitiveComponent Object Reference") (OtherActor :type "Actor Object Reference") (OtherComp :type "PrimitiveComponent Object Reference") (OtherBodyIndex :type Integer) (bFromSweep :type Boolean) (SweepResult :type "HitResult Structure (by ref)"))
  ;[1 1 1] When the player gets close to the weapon, UI is shown telling the player they can equip that weapon, as long as they are not already holding that type of weapon. When they move away, the UI is hidden.
  (bind _asthird_person_character (cast `/Game/StarterContent/ThirdPersonBP/Blueprints/ThirdPersonCharacter` OtherActor))
  (if (not (== (`/Game/StarterContent/ThirdPersonBP/Blueprints/ThirdPersonCharacter.WeaponMode` _asthird_person_character) 2))
    (set `/Game/StarterContent/ThirdPersonBP/Blueprints/ThirdPersonCharacter.NearSpear` true _asthird_person_character)
    (`SceneComponent.SetVisibility` (`self.PickupUI`) true false)))

(event `self.UI_DisplayZone.OnComponentEndOverlap`
  (params (OverlappedComponent :type "PrimitiveComponent Object Reference") (OtherActor :type "Actor Object Reference") (OtherComp :type "PrimitiveComponent Object Reference") (OtherBodyIndex :type Integer))
  ;[1 1 1] When the player gets close to the weapon, UI is shown telling the player they can equip that weapon, as long as they are not already holding that type of weapon. When they move away, the UI is hidden.
  (bind _asthird_person_character (cast `/Game/StarterContent/ThirdPersonBP/Blueprints/ThirdPersonCharacter` OtherActor))
  (set `/Game/StarterContent/ThirdPersonBP/Blueprints/ThirdPersonCharacter.NearSpear` false _asthird_person_character)
  (`SceneComponent.SetVisibility` (`self.PickupUI`) false false))

(fn `UserConstructionScript`)